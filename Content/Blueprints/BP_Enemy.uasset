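; BP_Enemy is a Paper2D enemy character with flipbook animation and a death sequence.
; AnyDamage checks Health minus Damage without storing the result; a lethal hit disables capsule collision, plays the non-looping Samurai death flipbook, then destroys the actor after a delay.
; NewFunction picks Fighter idle, walk or jump flipbooks from ground state and velocity, but nothing in this file calls it.
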(event `self.ReceiveBeginPlay`)

(event `self.ReceiveTick`
  (params (DeltaSeconds :type "Float (single-precision)")))

(event `self.ReceiveAnyDamage`
  (params (Damage :type "Float (single-precision)") (DamageType :type "DamageType Object Reference") (InstigatedBy :type "Controller Object Reference") (DamageCauser :type "Actor Object Reference"))
  (if (not (> (- (`self.Health`) Damage) 0.0))
    (`PrimitiveComponent.SetCollisionEnabled` (`self.CapsuleComponent`) "NoCollision")
    (`PaperFlipbookComponent.SetFlipbook` (`self.Sprite`) "/Game/PaperAssets/Character/Samurai/Filpbook_Samurai_Dead.Filpbook_Samurai_Dead")
    (`PaperFlipbookComponent.SetLooping` (`self.Sprite`) false)
    (`KismetSystemLibrary.Delay` 0.8)
    (`self.K2_DestroyActor`)))

(fn `NewFunction`
  (bind (_returnvalue_x _returnvalue_y _returnvalue_z) (`KismetMathLibrary.BreakVector` (`self.GetVelocity`)))
  (if (`NavMovementComponent.IsMovingOnGround` (`self.CharacterMovement`))
    (if (> (`KismetMathLibrary.VSize` (`self.GetVelocity`)) 0.0)
      (`PaperFlipbookComponent.SetFlipbook` (`self.Sprite`) "/Game/PaperAssets/Character/Fighter/Filpbook_Fighter_Walk.Filpbook_Fighter_Walk")
      (else
        (`PaperFlipbookComponent.SetFlipbook` (`self.Sprite`) "/Game/PaperAssets/Character/Fighter/Filpbook_Fighter_Idle.Filpbook_Fighter_Idle")))
    (elif (< _returnvalue_z -100.0)
      (`PaperFlipbookComponent.SetFlipbook` (`self.Sprite`) "/Game/PaperAssets/Character/Fighter/Filpbook_Fighter_Idle.Filpbook_Fighter_Idle")
      (else
        (`PaperFlipbookComponent.SetFlipbook` (`self.Sprite`) "/Game/PaperAssets/Character/Fighter/Filpbook_Fighter_Jump.Filpbook_Fighter_Jump")))))

(fn `UserConstructionScript`)